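; BP_StrangeDoor is a door that swings its static mesh 90 degrees in yaw and straight back each time DoorActivated fires.
; Two chained timelines lerp the world rotation out and back, storing DoorRotation after each swing, while CanAgain blocks re-triggering until both finish.
; BeginPlay is empty; the code that captures the initial rotation and starts a random-interval looping timer is disconnected, so nothing in this Blueprint triggers the door.
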(event Custom|DoorActivated
  (if (Variables|Default|GetCan%20Again)
    (Variables|Default|SetCan%20Again false)
    (bind _newtrack_0 (Timeline|Timeline PlayFromStart)
      (:Update
        (Transformation|SetWorldRotation (Variables|Default|GetStaticMesh) (Math|Rotator|Lerp(Rotator) (Variables|Default|GetDoorRotation) (Math|Rotator|MakeRotator (.Roll (Math|Rotator|BreakRotator (Variables|Default|GetDoorRotation))) (.Pitch (Math|Rotator|BreakRotator (Variables|Default|GetDoorRotation))) (- (.Yaw (Math|Rotator|BreakRotator (Variables|Default|GetDoorRotation))) 9e+01)) _newtrack_0) false false))
      (:Finished
        (Variables|Default|SetDoorRotation (Math|Rotator|Lerp(Rotator) (Variables|Default|GetDoorRotation) (Math|Rotator|MakeRotator (.Roll (Math|Rotator|BreakRotator (Variables|Default|GetDoorRotation))) (.Pitch (Math|Rotator|BreakRotator (Variables|Default|GetDoorRotation))) (- (.Yaw (Math|Rotator|BreakRotator (Variables|Default|GetDoorRotation))) 9e+01)) _newtrack_0))
        (bind _newtrack_0_2 (Timeline|Timeline_0 PlayFromStart)
          (:Update
            (Transformation|SetWorldRotation (Variables|Default|GetStaticMesh) (Math|Rotator|Lerp(Rotator) (Variables|Default|GetDoorRotation) (Math|Rotator|MakeRotator (.Roll (Math|Rotator|BreakRotator (Variables|Default|GetDoorRotation))) (.Pitch (Math|Rotator|BreakRotator (Variables|Default|GetDoorRotation))) (+ (.Yaw (Math|Rotator|BreakRotator (Variables|Default|GetDoorRotation))) 9e+01)) _newtrack_0_2) false false))
          (:Finished
            (Variables|Default|SetCan%20Again true)
            (Variables|Default|SetDoorRotation (Math|Rotator|Lerp(Rotator) (Variables|Default|GetDoorRotation) (Math|Rotator|MakeRotator (.Roll (Math|Rotator|BreakRotator (Variables|Default|GetDoorRotation))) (.Pitch (Math|Rotator|BreakRotator (Variables|Default|GetDoorRotation))) (+ (.Yaw (Math|Rotator|BreakRotator (Variables|Default|GetDoorRotation))) 9e+01)) _newtrack_0_2))))))))

(event EventBeginPlay)

(fn ConstructionScript)