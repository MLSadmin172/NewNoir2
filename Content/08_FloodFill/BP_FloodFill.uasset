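; Interactive cutout minigame actor where look input moves a cube cursor and holding input draws its path onto a canvas render target.
; On release, a GPU flood fill from a fixed seed runs fixed iterations of ping-ponged material draws between two render targets.
; If the center pixel stays unfilled, it spawns a BP_Photo with the canvas, destroys itself and spawns the next round until ID reaches 2.
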(event Input|EnhancedActionEvents|EnhancedInputActionIA_Hold
  (params (ActionValue :type Boolean) (ElapsedSeconds :type Float%20%28double-precision%29) (TriggeredSeconds :type Float%20%28double-precision%29) (InputAction :type Input%20Action%20Object%20Reference :default "/Game/FirstPerson/Input/Actions/IA_Hold.IA_Hold"))
  (bind _cube1 (Variables|Default|GetCube1))
  (bind _relativelocation (Variables|/Script/Engine.SceneComponent|GetRelativeLocation _cube1))
  (bind _returnvalue (+ (.z _relativelocation) 5e+01))
  (bind _returnvalue_2 (+ (.x _relativelocation) 5e+01))
  (bind _returnvalue_3 (/ _returnvalue_2 1e+02))
  (bind _returnvalue_4 (/ _returnvalue 1e+02))
  (bind _returnvalue_5 (* _returnvalue_3 256.0))
  (bind _returnvalue_6 (- 1.0 _returnvalue_4))
  (bind _returnvalue_7 (* _returnvalue_6 256.0))
  (bind _returnvalue_8 (Math|Vector2D|MakeVector2D _returnvalue_5 _returnvalue_7))
  (:Triggered
    (bind _canvas (Rendering|BeginDrawCanvastoRenderTarget (Variables|Default|GetCanvas)))
    (if (Utilities|Operators|NotEqual(!=) :A (Variables|Default|GetLastPos))
      (Class|Canvas|DrawLine _canvas (Variables|Default|GetLastPos) _returnvalue_8 1.0 "(R=0.000000,G=0.000000,B=1.000000,A=1.000000)"))
    (Variables|Default|SetLastPos _returnvalue_8))
  (:Started
    (Rendering|Material|SetVectorParameterValue (Variables|DMI|GetDMI_Finish) "FillColor" (Variables|Default|GetClearColor) :!class /Script/Engine.MaterialInstanceDynamic)
    (CallFunction|DoFill))
  (:Completed
    (Rendering|Material|SetVectorParameterValue (Variables|DMI|GetDMI_Finish) "FillColor" (Variables|Default|GetFillColor) :!class /Script/Engine.MaterialInstanceDynamic)
    (CallFunction|DoFill)
    (bind _returnvalue_9 (Class|KismetRenderingLibrary|ReadRenderTargetUV (Variables|Default|GetCanvas) 0.5 0.5))
    (if (not (== (.r (Math|Conversions|ToLinearColor(Color) _returnvalue_9)) 1.0))
      (Rendering|Material|SetVectorParameterValue (Variables|DMI|GetDMI_Finish) "FillColor" "(R=1.000000,G=1.000000,B=1.000000,A=1.000000)" :!class /Script/Engine.MaterialInstanceDynamic)
      (CallFunction|DoFill)
      (CallFunction|ManualStop)
      (Actor|DestroyActor)
      (Game|SpawnActorfromClass "/Game/FirstPerson/Blueprints/Items/BP_Photo.BP_Photo_C" (Transformation|GetActorTransform (Variables|Default|GetPhotoSpawnPos)) "Undefined" "MultiplyWithRoot" 0 (Variables|Default|GetCanvas) (Variables|Default|GetID) 0)
      (if (< (Variables|Default|GetID) 2)
        (Game|SpawnActorfromClass "BP_FloodFill_C" (Transformation|GetActorTransform) "Undefined" "MultiplyWithRoot" 0 (Variables|Default|GetPhotoSpawnPos) (+ (Variables|Default|GetID) 1) 0)))))

(event EventBeginPlay
  (Rendering|ClearRenderTarget2D (Variables|Default|GetCanvas)))

(event EventStartInteraction
  (Game|Player|SetViewTargetwithBlend (Game|GetPlayerController 0) self 0.2 "VTBlend_Linear" 0.0 false))

(event EventStopInteraction
  (Game|Player|SetViewTargetwithBlend (Game|GetPlayerController 0) (Game|GetPlayerCharacter 0) 0.2 "VTBlend_Linear" 0.0 false))

(event EventTick
  (params (DeltaSeconds :type Float%20%28single-precision%29))
  (bind _returnvalue (Input|EnhancedActionValues|GetIA_Look))
  (bind _cube1 (Variables|Default|GetCube1))
  (bind _relativelocation (Variables|/Script/Engine.SceneComponent|GetRelativeLocation _cube1))
  (if (Variables|Default|GetInteracting)
    (Transformation|SetRelativeLocation _cube1 (Math|Vector|MakeVector (Math|Float|Clamp(Float) (+ (.x _returnvalue) (.x _relativelocation)) -3e+01 3e+01) 0.0 (Math|Float|Clamp(Float) (+ (.z _relativelocation) (* (.y _returnvalue) -1.0)) -3e+01 3e+01)) false false)))

(fn ConstructionScript
  (Utilities|FlowControl|Sequence
    (:then_0
      (bind _returnvalue (Rendering|CreateRenderTarget2D 256 256 "RTF_RGBA8_SRGB"))
      (Variables|Default|SetCanvas _returnvalue))
    (:then_1
      ;[1 1 1] Create Render Targets with the correct size
      (bind _returnvalue_2 (Rendering|CreateRenderTarget2D (Variables|/Script/Engine.TextureRenderTarget2D|GetSizeX (Variables|Default|GetCanvas)) (Variables|/Script/Engine.TextureRenderTarget2D|GetSizeY (Variables|Default|GetCanvas)) "RTF_R8" "(R=0.000000,G=1.000000,B=0.000000,A=1.000000)"))
      (Variables|RenderTargets|SetRT1 _returnvalue_2)
      (bind _returnvalue_3 (Rendering|CreateRenderTarget2D (Variables|/Script/Engine.TextureRenderTarget2D|GetSizeX (Variables|Default|GetCanvas)) (Variables|/Script/Engine.TextureRenderTarget2D|GetSizeY (Variables|Default|GetCanvas)) "RTF_R8" "(R=0.000000,G=1.000000,B=0.000000,A=1.000000)"))
      (Variables|RenderTargets|SetRT2 _returnvalue_3)
      (bind _returnvalue_4 (Rendering|CreateRenderTarget2D (Variables|/Script/Engine.TextureRenderTarget2D|GetSizeX (Variables|Default|GetCanvas)) (Variables|/Script/Engine.TextureRenderTarget2D|GetSizeY (Variables|Default|GetCanvas)) "RTF_RGBA8" "(R=1.000000,G=0.000000,B=0.629179,A=1.000000)"))
      (Variables|RenderTargets|SetRTResult _returnvalue_4)
      (bind _returnvalue_5 (Rendering|CreateRenderTarget2D (Variables|/Script/Engine.TextureRenderTarget2D|GetSizeX (Variables|Default|GetCanvas)) (Variables|/Script/Engine.TextureRenderTarget2D|GetSizeY (Variables|Default|GetCanvas)) "RTF_RGBA8" "(R=1.000000,G=0.000000,B=0.629179,A=1.000000)"))
      (Variables|RenderTargets|SetRTTemp _returnvalue_5))
    (:then_2
      ;[1 1 1] Create all needed Dynamic Material Instances
      (bind _returnvalue_6 (Rendering|Material|CreateDynamicMaterialInstance (Variables|Materials|GetInitMaterial) "None" "None" :!class /Script/Engine.KismetMaterialLibrary))
      (Variables|DMI|SetDMI_Init _returnvalue_6)
      (bind _returnvalue_7 (Rendering|Material|CreateDynamicMaterialInstance (Variables|Materials|GetViewMaterial) "None" "None" :!class /Script/Engine.KismetMaterialLibrary))
      (Variables|DMI|SetDMI_View _returnvalue_7)
      (bind _returnvalue_8 (Rendering|Material|CreateDynamicMaterialInstance (Variables|Materials|GetIterationMaterial) "None" "None" :!class /Script/Engine.KismetMaterialLibrary))
      (Variables|DMI|SetDMI_Iteration _returnvalue_8)
      (bind _returnvalue_9 (Rendering|Material|CreateDynamicMaterialInstance (Variables|Materials|GetFinishMaterial) "None" "None" :!class /Script/Engine.KismetMaterialLibrary))
      (Variables|DMI|SetDMI_Finish _returnvalue_9)
      (bind _returnvalue_10 (Rendering|Material|CreateDynamicMaterialInstance "/Game/02_ScalingKernel/M_CompositePaper.M_CompositePaper" "None" "None" :!class /Script/Engine.KismetMaterialLibrary))
      (Variables|Default|SetDMI_Comp _returnvalue_10))
    (:then_3
      ;[1 1 1] Set fill color. Set the tolerance for how much pixels have to match the color where the fill started to receive filing themselves.
      (Rendering|Material|SetScalarParameterValue (Variables|DMI|GetDMI_Iteration) "Tolerance" (Variables|Default|GetTolerance) :!class /Script/Engine.MaterialInstanceDynamic)
      (Rendering|Material|SetVectorParameterValue (Variables|DMI|GetDMI_Finish) "FillColor" (Variables|Default|GetFillColor) :!class /Script/Engine.MaterialInstanceDynamic))
    (:then_5
      ;[1 1 1] Set input texture in materials
      (Rendering|Material|SetTextureParameterValue (Variables|DMI|GetDMI_View) "InputTexture" (Variables|Default|GetCanvas))
      (Rendering|Material|SetTextureParameterValue (Variables|DMI|GetDMI_Init) "InputTexture" (Variables|Default|GetCanvas))
      (Rendering|Material|SetTextureParameterValue (Variables|DMI|GetDMI_Iteration) "StartTexture" (Variables|Default|GetCanvas))
      (Rendering|Material|SetTextureParameterValue (Variables|DMI|GetDMI_Finish) "InputTexture" (Variables|Default|GetCanvas))
      (Rendering|Material|SetTextureParameterValue (Variables|Default|GetDMI_Comp) "InputTexture" (Variables|Default|GetCanvas)))
    (:then_6
      ;[1 1 1] Set the view material on the plane
      (Rendering|Material|SetMaterial (Variables|Default|GetPlane) 0 (Variables|Default|GetDMI_Comp)))))

(fn DoFill
  (bind _returnvalue (Math|Conversions|ToLinearColor(Vector) "0, 0, 0"))
  (bind _canvas (Variables|Default|GetCanvas))
  (bind _dmi_view (Variables|DMI|GetDMI_View))
  (bind _rttemp (Variables|RenderTargets|GetRTTemp))
  (bind _dmi_finish (Variables|DMI|GetDMI_Finish))
  (bind _dmi_iteration (Variables|DMI|GetDMI_Iteration))
  (Utilities|FlowControl|Sequence
    (:then_0
      ;[1 1 1] Clear the RTs for a new floodfill mask
      (Rendering|ClearRenderTarget2D (Variables|RenderTargets|GetRT1))
      (Rendering|ClearRenderTarget2D (Variables|RenderTargets|GetRT2)))
    (:then_1
      ;[1 1 1] Setting material parameters before looping
      (Rendering|Material|SetVectorParameterValue (Variables|DMI|GetDMI_Init) "SeedPos" _returnvalue :!class /Script/Engine.MaterialInstanceDynamic)
      (Rendering|Material|SetVectorParameterValue (Variables|DMI|GetDMI_Iteration) "SeedPos" _returnvalue :!class /Script/Engine.MaterialInstanceDynamic)
      ;;[1 1 1] Writing to RT2 and setting it as input on the iteration material because the loop below starts with writing to RT1.. Thereby starting with RT2 as input
      (Rendering|DrawMaterialtoRenderTarget (Variables|RenderTargets|GetRT2) (Variables|DMI|GetDMI_Init))
      (Rendering|Material|SetTextureParameterValue (Variables|DMI|GetDMI_Iteration) "InputTexture" (Variables|RenderTargets|GetRT2)))
    (:then_2
      ;[1 1 1] Run the fill iteration a set number of times. When running on the GPU, because it is so parallelized, there is no easy way to sum up the pixels and see if you have done all the iterations you needed or if change still happens
      (for _index (range 0 (Variables|Default|GetFillIterations))
        (Rendering|DrawMaterialtoRenderTarget (Utilities|Select :Index (Math|Integer|%(Integer) _index 2) :Option%200 (Variables|RenderTargets|GetRT1) :Option%201 (Variables|RenderTargets|GetRT2)) _dmi_iteration)
        (Rendering|Material|SetTextureParameterValue _dmi_iteration "InputTexture" (Utilities|Select :Index (Math|Integer|%(Integer) _index 2) :Option%200 (Variables|RenderTargets|GetRT1) :Option%201 (Variables|RenderTargets|GetRT2)))))
    (:then_3
      ;[1 1 1] Set Finish Material parms, render to temp. finish buffer, switch and render to finish (Since we can't both read and write to finish)
      (Rendering|Material|SetTextureParameterValue (Variables|DMI|GetDMI_Finish) "MaskTexture" (Utilities|Select :Index (Math|Integer|%(Integer) (Variables|Default|GetFillIterations) 2) :Option%200 (Variables|RenderTargets|GetRT1) :Option%201 (Variables|RenderTargets|GetRT2)))
      (Rendering|DrawMaterialtoRenderTarget _rttemp _dmi_finish)
      (Rendering|Material|SetTextureParameterValue _dmi_finish "InputTexture" _rttemp)
      (Rendering|DrawMaterialtoRenderTarget (Variables|RenderTargets|GetRTResult) _dmi_finish))
    (:then_4
      ;[1 1 1] Set input texture in materials
      (Rendering|Material|SetTextureParameterValue _dmi_view "InputTexture" (Variables|RenderTargets|GetRTResult))
      (Rendering|DrawMaterialtoRenderTarget _canvas _dmi_view)
      (Rendering|Material|SetTextureParameterValue (Variables|DMI|GetDMI_View) "InputTexture" _canvas)
      (Rendering|Material|SetTextureParameterValue (Variables|DMI|GetDMI_Iteration) "StartTexture" _canvas)
      (Rendering|Material|SetTextureParameterValue (Variables|DMI|GetDMI_Finish) "InputTexture" _canvas))))

(fn GetLocalCursorPosition)